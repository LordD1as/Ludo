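; Game instance for the Ludo game that responds to online session results.
; On Init it waits briefly, then binds handlers to the session subsystem's create, join and find-friend-session completion events.
; A created session opens the Lobby as a listen server, and a successful join runs an open console command with the returned address.
; Failures show an error widget; a successful friend search triggers nothing here.
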(event `self.ReceiveInit`
  (`KismetSystemLibrary.Delay` 1.0)
  (add `SessionSubsystem.OnCreateSessionCompleteEvent` (subsystem `SessionSubsystem`) (delegate `OnCreateSessionCompleted`))
  (add `SessionSubsystem.OnJoinGameSessionCompleteEvent` (subsystem `SessionSubsystem`) (delegate `OnJoinSessionCompleteEvent`))
  (add `SessionSubsystem.OnFindFriendSessionCompleteEvent` (subsystem `SessionSubsystem`) (delegate `OnFindFriendSessionCompleteEvent`)))

(event `OnJoinSessionCompleteEvent`
  (params (JoinResult :type "EJoinResultType Enum" :default "Success") (Address :type String))
  (switch `EJoinResultType` JoinResult
    (:`Success`
      (`KismetSystemLibrary.ExecuteConsoleCommand` (`KismetStringLibrary.Concat_StrStr` "open " Address) (`GameplayStatics.GetPlayerController` 0)))
    (:`SessionIsFull`
      (`self.OnShowWidget` (make `WidgetState` "ErrorMsg" "Failed to join session.") :!label _label))
    (:`SessionDoesNotExist`
      (goto _label))
    (:`CouldNotRetrieveAddress`
      (goto _label))
    (:`AlreadyInSession`
      (goto _label))
    (:`UnknownError`
      (goto _label))))

(event `OnFindFriendSessionCompleteEvent`
  (params (LocalUserNum :type Integer) (bWasSuccessful :type Boolean) (SessionResults :type "Array of BlueprintSessionResult Structure (by ref)"))
  (if (not bWasSuccessful)
    (`self.OnShowWidget` (make `WidgetState` "ErrorMsg" "Couldn't find session to rejoin."))))

(event `OnCreateSessionCompleted`
  (params (Successful :type Boolean))
  (if Successful
    (`GameplayStatics.OpenLevelBySoftObjectPtr` "/Game/Maps/Lobby.Lobby" true "?listen")
    (else
      (`self.OnShowWidget` (make `WidgetState` "ErrorMsg")))))